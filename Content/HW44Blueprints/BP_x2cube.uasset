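; Actor that continuously spins two cube components on different axes.
; BeginPlay caches both relative rotations, then starts the Rotator timeline, which restarts itself each time it finishes.
; Each update lerps from the cached rotations: Cube toward 360 yaw using its current roll and pitch, Cube1 through a full added pitch turn.
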(event Custom|Rotate
  (bind _cube (Variables|Default|GetCube))
  (bind _rr2 (Variables|Default|GetRR2))
  (bind _relativerotation (Variables|/Script/Engine.SceneComponent|GetRelativeRotation _cube))
  (bind _alpha (Timeline|Rotator PlayFromStart)
    (:Update
      (Transformation|SetRelativeRotation _cube (Math|Rotator|Lerp(Rotator) (Variables|Default|GetRR1) (Math|Rotator|MakeRotator (.roll _relativerotation) (.pitch _relativerotation) 3.6e+02) _alpha) false false)
      (Transformation|SetRelativeRotation (Variables|Default|GetCube1) (Math|Rotator|Lerp(Rotator) (Variables|Default|GetRR2) (Math|Rotator|MakeRotator (.roll _rr2) (+ (.pitch _rr2) 3.6e+02) (.yaw _rr2)) _alpha) false false))
    (:Finished
      (CallFunction|Rotate))))

(event EventBeginPlay
  (Variables|Default|SetRR1 (Variables|/Script/Engine.SceneComponent|GetRelativeRotation (Variables|Default|GetCube)))
  (Variables|Default|SetRR2 (Variables|/Script/Engine.SceneComponent|GetRelativeRotation (Variables|Default|GetCube1)))
  (CallFunction|Rotate))

(fn ConstructionScript)